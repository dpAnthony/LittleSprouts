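; Floating name label actor that displays the name of the MyBaby actor at that actor's position.
; On BeginPlay it caches the first MyBaby found in the level.
; Every Tick it snaps to the baby's location, without inheriting rotation or scale, and refreshes its TextRender with BabyName.
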(event EventBeginPlay
  (bind _outactors (Actor|GetAllActorsOfClass "/Game/Blueprints/myBaby.myBaby_C"))
  (Variables|Default|SetmyBabyRef (Utilities|Array|Get(acopy) _outactors)))

(event Collision|EventActorBeginOverlap
  (params (OtherActor :type Actor%20Object%20Reference)))

(event EventTick
  (params (DeltaSeconds :type Float%20%28single-precision%29))
  (Transformation|SetActorTransform (Math|Conversions|ToTransform(Vector) (.Location (Math|Transform|BreakTransform (Transformation|GetActorTransform (Variables|Default|GetmyBabyRef))))))
  (Rendering|Components|TextRender|SetText (Variables|Default|GetTextRender) (Utilities|Text|ToText(String) (Variables|/Game/Blueprints/myBaby.myBaby_C|GetbabyName (Variables|Default|GetmyBabyRef)))))

(fn ConstructionScript)
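; Clickable hazard actor with a configurable mesh, an info menu and an optional scenario card.
; Hovering outlines the mesh via custom depth; clicking outside the baby's turn moves the player pawn to it, then shows the menu.
; Its hit box is sized from mesh bounds plus padding.
; When a baby AI targeting it hits that box on its turn, or ShowScenario fires, the scenario card appears and the game pauses.
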(event OnClicked(staticMesh)
  (params (TouchedComponent :type Primitive%20Component%20Object%20Reference) (ButtonPressed :type Key%20Structure))
  (bind _widgetreference (Variables|Default|GetwidgetReference))
  ;[1 1 1] Smooth Move CameraPawn to Hazard
  (bind _asplayer_pawn_ctrl (Utilities|Casting|CastToPlayerPawnCtrl (Game|GetPlayerController 0)))
  (if (not (Variables|/Game/TopDownBP/Blueprints/PlayerPawnCtrl.PlayerPawnCtrl_C|GetBabysTurn _asplayer_pawn_ctrl))
    (Default|MovePawnInit _asplayer_pawn_ctrl (Transformation|GetActorLocation))
    (Default|MovePawntoHazard _asplayer_pawn_ctrl)
    (Utilities|FlowControl|Delay 0.7)
    (if (Variables|Default|GethasWidget)
      (Widget|SetVisibility _widgetreference "Visible")
      (Default|InitAnim _widgetreference)
      (else
        (UserInterface|Viewport|AddtoViewport _widgetreference 0)
        (Widget|SetVisibility _widgetreference "Visible")
        (Default|InitAnim _widgetreference)
        (Variables|Default|SethasWidget true)))))

(event OnEndCursorOver(staticMesh)
  (params (TouchedComponent :type Primitive%20Component%20Object%20Reference))
  (Rendering|SetRenderCustomDepth (Variables|Mesh|GetStaticMesh) false))

(event OnComponentHit(HitCollision)
  (params (HitComponent :type Primitive%20Component%20Object%20Reference) (OtherActor :type Actor%20Object%20Reference) (OtherComp :type Primitive%20Component%20Object%20Reference) (NormalImpulse :type Vector :default "0, 0, 0") (Hit :type Hit%20Result%20Structure%20%28by%20ref%29))
  (bind _scenarioreference (Variables|Default|GetscenarioReference))
  ;[1 1 1] Check if other object is baby, if so open dialogue
  (if (Variables|Default|GethasScenario)
    (Variables|Default|SetLocalBabyRef OtherActor)
    (bind _asplayer_pawn_ctrl (Utilities|Casting|CastToPlayerPawnCtrl (Game|GetPlayerController 0)))
    (if (Variables|/Game/TopDownBP/Blueprints/PlayerPawnCtrl.PlayerPawnCtrl_C|GetBabysTurn _asplayer_pawn_ctrl)
      (bind _asmy_baby_ai (Utilities|Casting|CastTomyBabyAi (Variables|Default|GetLocalBabyRef)))
      (if (== (Variables|/Game/Blueprints/myBabyAi.myBabyAi_C|GetCurrentTarget _asmy_baby_ai) self)
        (bind _asmy_baby_ai_2 (Utilities|Casting|CastTomyBabyAi (Variables|Default|GetLocalBabyRef)))
        (Variables|/Game/Blueprints/myBabyAi.myBabyAi_C|SetCurrentTarget _asmy_baby_ai_2 0)
        (Variables|/Game/Blueprints/myBabyAi.myBabyAi_C|SetfaceVar _asmy_baby_ai_2 2)
        (Widget|SetVisibility _scenarioreference "Visible")
        (Input|SetInputModeUIOnly (Game|GetPlayerController 0) _scenarioreference "DoNotLock")
        (Game|SetGamePaused true)))))

(event OnBeginCursorOver(staticMesh)
  (params (TouchedComponent :type Primitive%20Component%20Object%20Reference))
  (Rendering|SetRenderCustomDepth (Variables|Mesh|GetStaticMesh) true))

(event Custom|SetHitCollisionBounds
  (bind _hitcollision (Variables|Default|GetHitCollision))
  ;[1 1 1] Resize Collision Bounds
  (Variables|/Script/Engine.SceneComponent|SetbAbsoluteScale _hitcollision true)
  (Components|Box|SetBoxExtent _hitcollision (+ (.Max (Components|StaticMesh|GetLocalBounds (Variables|Default|GetstaticMesh))) "30.000000,30.000000,50.000000") true))

(event Custom|ShowScenario
  (bind _scenarioreference (Variables|Default|GetscenarioReference))
  (if (Variables|Default|GethasScenario)
    (Game|SetGamePaused true)
    (Widget|SetVisibility _scenarioreference "Visible")
    (Input|SetInputModeUIOnly (Game|GetPlayerController 0) _scenarioreference "DoNotLock")))

(event EventBeginPlay
  ;[1 1 1] Init Hazard Menu
  (bind _returnvalue (UserInterface|CreateWidget "/Game/UI_Widgets/HazardMenu.HazardMenu_C" (Game|GetPlayerController 0)))
  (bind _output_get (Variables|Default|SetwidgetReference _returnvalue))
  (Variables|/Game/UI_Widgets/HazardMenu.HazardMenu_C|SetobjName _output_get (Variables|Default|GetobjectName))
  (Variables|/Game/UI_Widgets/HazardMenu.HazardMenu_C|SetobjDesc _output_get (Variables|Default|GetobjectDescription))
  (CallFunction|SetHitCollisionBounds)
  (if (Variables|Default|GethasScenario)
    (bind _returnvalue_2 (UserInterface|CreateWidget "/Game/UI_Widgets/ScenarioCard.ScenarioCard_C" (Game|GetPlayerController 0)))
    (bind _output_get_2 (Variables|Default|SetscenarioReference _returnvalue_2))
    (Default|SetText _output_get_2 (Variables|Default|GetscenarioName) (Variables|Default|GetscenarioText))
    (UserInterface|Viewport|AddtoViewport _output_get_2 0)
    (Widget|SetVisibility _output_get_2 "Collapsed")))

(fn ConstructionScript
  (Components|StaticMesh|SetStaticMesh (Variables|Default|GetstaticMesh) (Variables|Default|GetvariableMesh)))
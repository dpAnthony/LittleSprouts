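; AudioManager actor that switches background music between the main menu, gameplay levels and game over.
; BeginPlay creates three audio components for those tracks and stops them.
; Tick polls CurrentLevelName on PlayerPawnCtrl and crossfades to the matching track, with Levels 1 to 3 sharing LevelMusic.
; Each case has its own never-reset DoOnce, so each fades once per actor lifetime and each numbered level calls FadeIn separately.
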(event EventBeginPlay
  (bind _returnvalue (AddComponent|AddAudioComponent false))
  (bind _output_get (Variables|Default|SetMainMenuMusic _returnvalue))
  (Audio|Components|Audio|Stop _output_get)
  (bind _returnvalue_2 (AddComponent|AddAudioComponent false))
  (bind _output_get_2 (Variables|Default|SetLevelMusic _returnvalue_2))
  (Audio|Components|Audio|Stop _output_get_2)
  (bind _returnvalue_3 (AddComponent|AddAudioComponent false))
  (bind _output_get_3 (Variables|Default|SetGameOverMusic _returnvalue_3))
  (Audio|Components|Audio|Stop _output_get_3))

(event EventTick
  (params (DeltaSeconds :type Float%20%28single-precision%29))
  (bind _asplayer_pawn_ctrl (Utilities|Casting|CastToPlayerPawnCtrl (Game|GetPlayerController 0)))
  (switch string (Variables|/Game/TopDownBP/Blueprints/PlayerPawnCtrl.PlayerPawnCtrl_C|GetCurrentLevelName _asplayer_pawn_ctrl)
    (:PersistentLevel
      (Utilities|FlowControl|DoOnce false
        (:Completed
          (Audio|Components|Audio|FadeIn (Variables|Default|GetMainMenuMusic) 2.0 1.0 0.0 :!class /Script/Engine.AudioComponent))))
    (:Level1
      (Utilities|FlowControl|DoOnce false
        (:Completed
          (Audio|Components|Audio|FadeOut (Variables|Default|GetMainMenuMusic) 2.0 0.0 :!class /Script/Engine.AudioComponent)
          (Audio|Components|Audio|FadeIn (Variables|Default|GetLevelMusic) 2.0 1.0 0.0 :!class /Script/Engine.AudioComponent))))
    (:Level2
      (Utilities|FlowControl|DoOnce false
        (:Completed
          (Audio|Components|Audio|FadeOut (Variables|Default|GetMainMenuMusic) 2.0 0.0 :!class /Script/Engine.AudioComponent)
          (Audio|Components|Audio|FadeIn (Variables|Default|GetLevelMusic) 2.0 1.0 0.0 :!class /Script/Engine.AudioComponent))))
    (:Level3
      (Utilities|FlowControl|DoOnce false
        (:Completed
          (Audio|Components|Audio|FadeOut (Variables|Default|GetMainMenuMusic) 2.0 0.0 :!class /Script/Engine.AudioComponent)
          (Audio|Components|Audio|FadeIn (Variables|Default|GetLevelMusic) 2.0 1.0 0.0 :!class /Script/Engine.AudioComponent))))
    (:GameOver
      (Utilities|FlowControl|DoOnce false
        (:Completed
          (Audio|Components|Audio|FadeOut (Variables|Default|GetLevelMusic) 0.75 0.0 :!class /Script/Engine.AudioComponent)
          (Audio|Components|Audio|FadeIn (Variables|Default|GetGameOverMusic) 0.75 1.0 0.0 :!class /Script/Engine.AudioComponent))))))

(fn ConstructionScript)
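; AI baby pawn built from layered sprite planes, with clickable bounce reactions and custom-depth hover highlighting.
; ChangeVariable applies skin, hair and eye materials and saves the look and name to MyGameInstance.
; Random Tick checks trigger blinks and refresh the expression from FaceVar, which Bounce sets to surprise or laugh.
; BabyMovement wanders between random reachable navmesh points via AIMoveTo with debug spheres, while MoveToTarget follows a target actor.
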(event OnBeginCursorOver(0_headPlane)
  (params (TouchedComponent :type Primitive%20Component%20Object%20Reference))
  (Rendering|SetRenderCustomDepth TouchedComponent true))

(event OnEndCursorOver(0_headPlane)
  (params (TouchedComponent :type Primitive%20Component%20Object%20Reference))
  (Rendering|SetRenderCustomDepth TouchedComponent false))

(event Custom|MoveToTarget
  (params (Delta%20Seconds :type Float%20%28single-precision%29))
  ;[1 1 1] Move to Actor
  (AI|AIMoveTo self "0, 0, 0" (Variables|Default|GetCurrentTarget) 5.0 true))

(event Custom|Bounce
  ;[1 1 1] Bounce Anim
  (if (>= (Math|Random|RandomIntegerinRange 0 10) 5)
    (Variables|Default|SetfaceVar 4.0)
    (bind _bounce (Timeline|BounceClick PlayFromStart)
      (:Update
        (Transformation|SetActorScale3D _bounce)
        (Development|PrintString "Baby touch"))
      (:Finished
        (Variables|Default|SetfaceVar 0.0)))
    (else
      (Variables|Default|SetfaceVar 7.0)
      (Timeline|BounceClick PlayFromStart))))

(event Custom|Event%20Baby%20Movement
  ;[1 1 1] Random Movement Function
  (if (not (Variables|Default|GetisMoving))
    (if (not (Variables|Default|GetIdle))
      (bind _outactors (Actor|GetAllActorsOfClass "/Script/Engine.RecastNavMesh"))
      (bind _output_get (Variables|Default|SetCurrentTargetLoc (.RandomLocation (AI|Navigation|GetRandomReachablePointinRadius (Transformation|GetActorLocation) (Variables|Default|GetmoveRadius) (Utilities|Array|Get(acopy) _outactors) "/Script/Engine.RecastFilter_UseDefaultArea"))))
      (Rendering|Debug|DrawDebugSphere _output_get 1e+01 5 "(R=1.000000,G=0.654150,B=0.211286,A=1.000000)" 9999999999.0)
      (AI|AIMoveTo self _output_get 0 15.0 false
        (:then
          (Development|PrintString "is moving")
          (Variables|Default|SetisMoving true))
        (:OnSuccess
          (Development|PrintString "got there")
          (Variables|Default|SetisMoving false :!label _label)
          (Utilities|FlowControl|Delay (Math|Random|RandomFloatinRange 0.3 1.0))
          (CallFunction|EventBabyMovement))
        (:OnFail
          (Development|PrintString "couldnt get there")
          (goto _label))))))

(event Custom|Blink
  ;[1 1 1] Blink
  (Rendering|SetVisibility (Variables|Default|Get2_eyePlane) false false)
  (Rendering|SetVisibility (Variables|Default|Get2_blinkPlane) true false)
  (Utilities|FlowControl|Delay (Math|Random|RandomFloatinRange 0.1 0.25))
  (Rendering|SetVisibility (Variables|Default|Get2_eyePlane) true false)
  (Rendering|SetVisibility (Variables|Default|Get2_blinkPlane) false false))

(event EventBeginPlay
  ;[1 1 1] Init Baby
  (Variables|/Script/Engine.PlayerController|SetbEnableMouseOverEvents (Game|GetPlayerController 0) true)
  (Variables|/Script/Engine.SceneComponent|SetbAbsoluteScale (Variables|Collision|GetCapsuleComponent) true))

(event EventTick
  (params (DeltaSeconds :type Float%20%28single-precision%29))
  (bind _facevar (Variables|Default|GetfaceVar))
  (bind _3_expressionplane (Variables|Default|Get3_expressionPlane))
  (if (>= (Math|Random|RandomIntegerinRange 0 100) 90)
    (CallFunction|Blink)
    ;[1 1 1] Change Expression Sprite
    (if (== _facevar 0.0)
      (Rendering|Material|SetMaterial _3_expressionplane 0 "/Game/Materials/Baby/m_exp_happy.m_exp_happy")
      (elif (== _facevar 1.0)
        (Rendering|Material|SetMaterial _3_expressionplane 0 "/Game/Materials/Baby/m_exp_angry.m_exp_angry")
        (elif (== _facevar 2.0)
          (Rendering|Material|SetMaterial _3_expressionplane 0 "/Game/Materials/Baby/m_exp_sad.m_exp_sad")
          (elif (== _facevar 3.0)
            (Rendering|Material|SetMaterial _3_expressionplane 0 "/Game/Materials/Baby/m_exp_scared.m_exp_scared")
            (elif (== _facevar 4.0)
              (Rendering|Material|SetMaterial _3_expressionplane 0 "/Game/Materials/Baby/m_exp_surprise.m_exp_surprise")
              (elif (== _facevar 5.0)
                (Rendering|Material|SetMaterial _3_expressionplane 0 "/Game/Materials/Baby/m_exp_sleep.m_exp_sleep")
                (elif (== _facevar 6.0)
                  (Rendering|Material|SetMaterial _3_expressionplane 0 "/Game/Materials/Baby/m_exp_sleep2.m_exp_sleep2")
                  (elif (== _facevar 7.0)
                    (Rendering|Material|SetMaterial _3_expressionplane 0 "/Game/Materials/Baby/m_exp_laugh.m_exp_laugh")))))))))))

(fn ConstructionScript)

(fn ChangeVariable
  (params (g_hairVar :type Float%20%28single-precision%29) (g_skinVar :type Float%20%28single-precision%29) (g_faceVar :type Float%20%28single-precision%29) (g_eyeVar :type Float%20%28single-precision%29) (g_name :type String))
  (bind _0_headplane (Variables|Default|Get0_headPlane))
  (bind _2_eyeplane (Variables|Default|Get2_eyePlane))
  (bind _1_hairplane (Variables|Default|Get1_hairPlane))
  (Variables|Default|SethairVar g_hairVar)
  (Variables|Default|SetskinVar g_skinVar)
  (Variables|Default|SetfaceVar g_faceVar)
  (Variables|Default|SeteyeVar g_eyeVar)
  (Variables|Default|SetbabyName g_name)
  (Utilities|FlowControl|Sequence
    (:then_0
      ;[1 1 1] Change Head Sprite
      (if (== (Variables|Default|GetskinVar) 0.0)
        (Rendering|Material|SetMaterial _0_headplane 0 "/Game/Materials/Baby/m_skin1.m_skin1")
        (elif (== (Variables|Default|GetskinVar) 1.0)
          (Rendering|Material|SetMaterial _0_headplane 0 "/Game/Materials/Baby/m_skin2.m_skin2")
          (elif (== (Variables|Default|GetskinVar) 2.0)
            (Rendering|Material|SetMaterial _0_headplane 0 "/Game/Materials/Baby/m_skin3.m_skin3")
            (elif (== (Variables|Default|GetskinVar) 3.0)
              (Rendering|Material|SetMaterial _0_headplane 0 "/Game/Materials/Baby/m_skin4.m_skin4")
              (elif (== (Variables|Default|GetskinVar) 4.0)
                (Rendering|Material|SetMaterial _0_headplane 0 "/Game/Materials/Baby/m_skin5.m_skin5")
                (elif (== (Variables|Default|GetskinVar) 5.0)
                  (Rendering|Material|SetMaterial _0_headplane 0 "/Game/Materials/Baby/m_skin6.m_skin6"))))))))
    (:then_1
      ;[1 1 1] Change Hair Sprite
      (if (== (Variables|Default|GethairVar) 0.0)
        (Rendering|Material|SetMaterial _1_hairplane 0 "/Game/Materials/Baby/m_hair1.m_hair1")
        (elif (== (Variables|Default|GethairVar) 1.0)
          (Rendering|Material|SetMaterial _1_hairplane 0 "/Game/Materials/Baby/m_hair2.m_hair2")
          (elif (== (Variables|Default|GethairVar) 2.0)
            (Rendering|Material|SetMaterial _1_hairplane 0 "/Game/Materials/Baby/m_hair3.m_hair3")
            (elif (== (Variables|Default|GethairVar) 3.0)
              (Rendering|Material|SetMaterial _1_hairplane 0 "/Game/Materials/Baby/m_hair4.m_hair4")
              (elif (== (Variables|Default|GethairVar) 4.0)
                (Rendering|Material|SetMaterial _1_hairplane 0 "/Game/Materials/Baby/m_hair5.m_hair5")
                (elif (== (Variables|Default|GethairVar) 5.0)
                  (Rendering|Material|SetMaterial _1_hairplane 0 "/Game/Materials/Baby/m_hair6.m_hair6"))))))))
    (:then_2
      ;[1 1 1] Change Eye Sprite
      (if (== (Variables|Default|GeteyeVar) 0.0)
        (Rendering|Material|SetMaterial _2_eyeplane 0 "/Game/Materials/Baby/m_eyes1.m_eyes1")
        (elif (== (Variables|Default|GeteyeVar) 1.0)
          (Rendering|Material|SetMaterial _2_eyeplane 0 "/Game/Materials/Baby/m_eyes2.m_eyes2")
          (elif (== (Variables|Default|GeteyeVar) 2.0)
            (Rendering|Material|SetMaterial _2_eyeplane 0 "/Game/Materials/Baby/m_eyes3.m_eyes3")
            (elif (== (Variables|Default|GeteyeVar) 3.0)
              (Rendering|Material|SetMaterial _2_eyeplane 0 "/Game/Materials/Baby/m_eyes4.m_eyes4")
              (elif (== (Variables|Default|GeteyeVar) 4.0)
                (Rendering|Material|SetMaterial _2_eyeplane 0 "/Game/Materials/Baby/m_eyes5.m_eyes5")
                (elif (== (Variables|Default|GeteyeVar) 5.0)
                  (Rendering|Material|SetMaterial _2_eyeplane 0 "/Game/Materials/Baby/m_eyes6.m_eyes6"))))))))
    (:then_3
      (bind _asmy_game_instance (Utilities|Casting|CastToMyGameInstance (Game|GetGameInstance)))
      (Variables|/Game/TopDownBP/Blueprints/MyGameInstance.MyGameInstance_C|SetHairVar _asmy_game_instance (Variables|Default|GethairVar))
      (Variables|/Game/TopDownBP/Blueprints/MyGameInstance.MyGameInstance_C|SetSkinVar _asmy_game_instance (Variables|Default|GetskinVar))
      (Variables|/Game/TopDownBP/Blueprints/MyGameInstance.MyGameInstance_C|SetFaceVar _asmy_game_instance (Variables|Default|GetfaceVar))
      (Variables|/Game/TopDownBP/Blueprints/MyGameInstance.MyGameInstance_C|SetEyeVar _asmy_game_instance (Variables|Default|GeteyeVar))
      (Variables|/Game/TopDownBP/Blueprints/MyGameInstance.MyGameInstance_C|SetBabyName _asmy_game_instance (Variables|Default|GetbabyName)))))
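; Baby character built from layered sprite planes, with a random walk speed, name and swappable skin, hair, eye and expression materials.
; ChangeVariable stores the look and name and applies head, hair and eye materials, while Tick reapplies the expression from FaceVar.
; BabyMovement loops between random waits and AI moves to reachable nearby points; MoveToTarget pursues CurrentTarget.
; Cursor hover on the head toggles custom depth rendering.
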(event OnBeginCursorOver(0_headPlane)
  (params (TouchedComponent :type Primitive%20Component%20Object%20Reference))
  (Rendering|SetRenderCustomDepth TouchedComponent true))

(event OnEndCursorOver(0_headPlane)
  (params (TouchedComponent :type Primitive%20Component%20Object%20Reference))
  (Rendering|SetRenderCustomDepth TouchedComponent false))

(event Custom|MoveToTarget
  (params (Delta%20Seconds :type Float%20%28single-precision%29))
  ;[1 1 1] Move to Actor
  (AI|AIMoveTo self "0, 0, 0" (Variables|Default|GetCurrentTarget) 5.0 true))

(event Custom|Event%20Baby%20Movement
  (bind _returnvalue (Math|Random|RandomInteger 10))
  ;[1 1 1] Random Movement Function
  (if (not (Variables|Default|GetisMoving))
    (Development|PrintString (Utilities|String|ToString(Integer) _returnvalue))
    (if (<= _returnvalue 3)
      (Development|PrintString "Waiting")
      (Utilities|FlowControl|Delay (Math|Random|RandomFloatinRange 0.5 4.0))
      (CallFunction|EventBabyMovement)
      (else
        (AI|AIMoveTo self (.RandomLocation (AI|Navigation|GetRandomReachablePointinRadius (Transformation|GetActorLocation) (Variables|Default|GetmoveRadius))) 0 1e+01 false
          (:then
            (Variables|Default|SetisMoving true))
          (:OnSuccess
            (Variables|Default|SetisMoving false :!label _label)
            (CallFunction|EventBabyMovement))
          (:OnFail
            (goto _label)))))))

(event EventBeginPlay
  ;[1 1 1] Init Baby
  (Variables|/Script/Engine.PlayerController|SetbEnableMouseOverEvents (Game|GetPlayerController 0) true)
  (Utilities|FlowControl|Sequence
    (:then_0
      (bind _output_get (Variables|Default|SetmoveSpeed (Math|Random|RandomFloatinRange 5e+01 1e+02)))
      (Variables|/Script/Engine.CharacterMovementComponent|SetMaxWalkSpeed (Variables|Character|GetCharacterMovement) _output_get)
      (Transformation|SetActorRotation (Math|Rotator|MakeRotator (- 0.0 9e+01) 0.0 0.0)))))

(event EventTick
  (params (DeltaSeconds :type Float%20%28single-precision%29))
  (bind _facevar (Variables|Default|GetfaceVar))
  (bind _3_expressionplane (Variables|Default|Get3_expressionPlane))
  ;[1 1 1] Change Expression Sprite
  (if (== _facevar 0.0)
    (Rendering|Material|SetMaterial _3_expressionplane 0 "/Game/Materials/Baby/m_expression_1.m_expression_1")
    (elif (== _facevar 1.0)
      (Rendering|Material|SetMaterial _3_expressionplane 0 "/Game/Materials/Baby/m_expression_2.m_expression_2")
      (elif (== _facevar 2.0)
        (Rendering|Material|SetMaterial _3_expressionplane 0 "/Game/Materials/Baby/m_expression_3.m_expression_3")
        (elif (== _facevar 3.0)
          (Rendering|Material|SetMaterial _3_expressionplane 0 "/Game/Materials/Baby/m_expression_4.m_expression_4")
          (elif (== _facevar 4.0)
            (Rendering|Material|SetMaterial _3_expressionplane 0 "/Game/Materials/Baby/m_expression_5.m_expression_5")
            (elif (== _facevar 5.0)
              (Rendering|Material|SetMaterial _3_expressionplane 0 "/Game/Materials/Baby/m_expression_6.m_expression_6"))))))))

(fn ConstructionScript)

(fn ChangeVariable
  (params (g_hairVar :type Float%20%28single-precision%29) (g_skinVar :type Float%20%28single-precision%29) (g_faceVar :type Float%20%28single-precision%29) (g_eyeVar :type Float%20%28single-precision%29) (g_name :type String))
  (bind _0_headplane (Variables|Default|Get0_headPlane))
  (bind _2_eyeplane (Variables|Default|Get2_eyePlane))
  (bind _1_hairplane (Variables|Default|Get1_hairPlane))
  (Variables|Default|SethairVar g_hairVar)
  (Variables|Default|SetskinVar g_skinVar)
  (Variables|Default|SetfaceVar g_faceVar)
  (Variables|Default|SeteyeVar g_eyeVar)
  (bind _output_get (Variables|Default|SetbabyName g_name))
  (Utilities|FlowControl|Sequence
    (:then_0
      ;[1 1 1] Change Head Sprite
      (if (== (Variables|Default|GetskinVar) 0.0)
        (Rendering|Material|SetMaterial _0_headplane 0 "/Game/Materials/Baby/m_skin1.m_skin1")
        (elif (== (Variables|Default|GetskinVar) 1.0)
          (Rendering|Material|SetMaterial _0_headplane 0 "/Game/Materials/Baby/m_skin2.m_skin2")
          (elif (== (Variables|Default|GetskinVar) 2.0)
            (Rendering|Material|SetMaterial _0_headplane 0 "/Game/Materials/Baby/m_skin3.m_skin3")
            (elif (== (Variables|Default|GetskinVar) 3.0)
              (Rendering|Material|SetMaterial _0_headplane 0 "/Game/Materials/Baby/m_skin4.m_skin4")
              (elif (== (Variables|Default|GetskinVar) 4.0)
                (Rendering|Material|SetMaterial _0_headplane 0 "/Game/Materials/Baby/m_skin5.m_skin5")
                (elif (== (Variables|Default|GetskinVar) 5.0)
                  (Rendering|Material|SetMaterial _0_headplane 0 "/Game/Materials/Baby/m_skin6.m_skin6"))))))))
    (:then_1
      ;[1 1 1] Change Hair Sprite
      (if (== (Variables|Default|GethairVar) 0.0)
        (Rendering|Material|SetMaterial _1_hairplane 0 "/Game/Materials/Baby/m_hair1.m_hair1")
        (elif (== (Variables|Default|GethairVar) 1.0)
          (Rendering|Material|SetMaterial _1_hairplane 0 "/Game/Materials/Baby/m_hair2.m_hair2")
          (elif (== (Variables|Default|GethairVar) 2.0)
            (Rendering|Material|SetMaterial _1_hairplane 0 "/Game/Materials/Baby/m_hair3.m_hair3")
            (elif (== (Variables|Default|GethairVar) 3.0)
              (Rendering|Material|SetMaterial _1_hairplane 0 "/Game/Materials/Baby/m_hair4.m_hair4")
              (elif (== (Variables|Default|GethairVar) 4.0)
                (Rendering|Material|SetMaterial _1_hairplane 0 "/Game/Materials/Baby/m_hair5.m_hair5")
                (elif (== (Variables|Default|GethairVar) 5.0)
                  (Rendering|Material|SetMaterial _1_hairplane 0 "/Game/Materials/Baby/m_hair6.m_hair6"))))))))
    (:then_2
      ;[1 1 1] Change Eye Sprite
      (if (== (Variables|Default|GeteyeVar) 0.0)
        (Rendering|Material|SetMaterial _2_eyeplane 0 "/Game/Materials/Baby/m_eyes1.m_eyes1")
        (elif (== (Variables|Default|GeteyeVar) 1.0)
          (Rendering|Material|SetMaterial _2_eyeplane 0 "/Game/Materials/Baby/m_eyes2.m_eyes2")
          (elif (== (Variables|Default|GeteyeVar) 2.0)
            (Rendering|Material|SetMaterial _2_eyeplane 0 "/Game/Materials/Baby/m_eyes3.m_eyes3")
            (elif (== (Variables|Default|GeteyeVar) 3.0)
              (Rendering|Material|SetMaterial _2_eyeplane 0 "/Game/Materials/Baby/m_eyes4.m_eyes4")
              (elif (== (Variables|Default|GeteyeVar) 4.0)
                (Rendering|Material|SetMaterial _2_eyeplane 0 "/Game/Materials/Baby/m_eyes5.m_eyes5")
                (elif (== (Variables|Default|GeteyeVar) 5.0)
                  (Rendering|Material|SetMaterial _2_eyeplane 0 "/Game/Materials/Baby/m_eyes6.m_eyes6"))))))))))